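; Ball Blueprint that handles the visual and sound feedback of a ball that hits bricks and other objects.
; The construction script creates a dynamic material from M_Ball on the static mesh.
; BeginPlay activates a Niagara effect and binds the damage-change event, which tints that material green at a damage of one and red otherwise.
; Hits play a 2D bounce sound unless the other actor is a CBBrick.
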(event Custom|OnDamageChangeEvent
  (Rendering|Material|SetVectorParameterValue (Variables|Default|GetMaterial) "Color" (Math|Color|SelectColor "(R=0.016807,G=0.270498,B=0.078187,A=1.000000)" "(R=0.427083,G=0.000000,B=0.022368,A=1.000000)" (== (Variables|Default|GetBallDamage) 1)) :!class /Script/Engine.MaterialInstanceDynamic))

(event EventBeginPlay
  (Components|Activation|Activate (Variables|Default|GetNiagara) false)
  (EventDispatchers|AssignOnDamageChange (delegate Custom|OnDamageChangeEvent)))

(event Collision|EventHit
  (params (MyComp :type Primitive%20Component%20Object%20Reference) (Other :type Actor%20Object%20Reference) (OtherComp :type Primitive%20Component%20Object%20Reference) (bSelfMoved :type Boolean) (HitLocation :type Vector :default "0, 0, 0") (HitNormal :type Vector :default "0, 0, 0") (NormalImpulse :type Vector :default "0, 0, 0") (Hit :type Hit%20Result%20Structure%20%28by%20ref%29))
  (Utilities|Casting|CastToCBBrick Other
    (:CastFailed
      (Audio|PlaySound2D "/Game/Sound/SW_Bounce.SW_Bounce" 1.0 1.0 0.0 0 0))))

(fn ConstructionScript
  (bind _staticmesh (Variables|Default|GetStaticMesh)
    (:then
      (bind _returnvalue (Rendering|Material|CreateDynamicMaterialInstance _staticmesh 0 "/Game/Materials/M_Ball.M_Ball" "None" :!class /Script/Engine.PrimitiveComponent))
      (Variables|Default|SetMaterial _returnvalue))
    (:else)))