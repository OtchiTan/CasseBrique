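; BP_Brick is a brick actor whose color reflects its current health.
; The construction script creates a dynamic instance of M_Brick on the static mesh and stores it.
; At BeginPlay it binds to OnHealthChanged, and each change sets the material's Color parameter from the Colors array, indexed by Health minus one.
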(event Custom|OnHealthChanged_Event
  (Rendering|Material|SetVectorParameterValue (Variables|Default|GetMaterial) "Color" (Math|Conversions|ToLinearColor(Color) (Utilities|Array|Get(acopy) (Variables|Default|GetColors) (- (Variables|Default|GetHealth) 1))) :!class /Script/Engine.MaterialInstanceDynamic))

(event EventBeginPlay
  (EventDispatchers|AssignOnHealthChanged (delegate Custom|OnHealthChanged_Event)))

(fn ConstructionScript
  (bind _returnvalue (Rendering|Material|CreateDynamicMaterialInstance (Variables|Default|GetStaticMesh) 0 "/Game/Materials/M_Brick.M_Brick" "None" :!class /Script/Engine.PrimitiveComponent))
  (Variables|Default|SetMaterial _returnvalue))